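; Player pawn that flies relative to its camera and picks up, throws or fires items with two independent hands.
; Enhanced Input drives unswept location offsets, via combined or per-axis move actions, and rotates the root.
; Each hand's box overlap tracks "Grab"-tagged actors, which grab input snaps to that hand's sphere.
; A shared throw/shoot action calls LanzarHacha on a held bp_hacha or bp_revolver, then clears that hand's state.
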(event EventBeginPlay
  (bind _asplayer_controller (Utilities|Casting|CastToPlayerController (Pawn|GetController)))
  (Input|AddMappingContext (PlayerController|LocalPlayerSubsystems|GetEnhancedInputLocalPlayerSubsystem _asplayer_controller) "/Game/Game/core/input/im_editor.im_editor" 0 "(bIgnoreAllPressedKeysUntilRelease=True,bForceImmediately=False,bNotifyUserSettings=False)"))

(event Collision|EventActorBeginOverlap
  (params (OtherActor :type Actor%20Object%20Reference)))

(event EventTick
  (params (DeltaSeconds :type Float%20%28single-precision%29)))

(event OnComponentBeginOverlap(BoxGrabLeft)
  (params (OverlappedComponent :type Primitive%20Component%20Object%20Reference) (OtherActor :type Actor%20Object%20Reference) (OtherComp :type Primitive%20Component%20Object%20Reference) (OtherBodyIndex :type Integer) (bFromSweep :type Boolean) (SweepResult :type Hit%20Result%20Structure%20%28by%20ref%29))
  (if (Actor|ActorHasTag OtherActor "Grab")
    (Utilities|FlowControl|Sequence
      (:then_0
        (Variables|Default|SetPuedeAgarrarIzquierda true))
      (:then_1
        (Variables|Default|SetobjetoManoIzquierda OtherActor)))))

(event OnComponentBeginOverlap(BoxGrabRight)
  (params (OverlappedComponent :type Primitive%20Component%20Object%20Reference) (OtherActor :type Actor%20Object%20Reference) (OtherComp :type Primitive%20Component%20Object%20Reference) (OtherBodyIndex :type Integer) (bFromSweep :type Boolean) (SweepResult :type Hit%20Result%20Structure%20%28by%20ref%29))
  (if (Actor|ActorHasTag OtherActor "Grab")
    (Utilities|FlowControl|Sequence
      (:then_0
        (Variables|Default|SetobjetoManoDerecha OtherActor)
        (Development|PrintString "Hacha lista para agarrar con la derecha"))
      (:then_1
        (Variables|Default|SetPuedeAgarrarDerecha true)))))

(event OnComponentEndOverlap(BoxGrabRight)
  (params (OverlappedComponent :type Primitive%20Component%20Object%20Reference) (OtherActor :type Actor%20Object%20Reference) (OtherComp :type Primitive%20Component%20Object%20Reference) (OtherBodyIndex :type Integer))
  (if (== (Variables|Default|GetobjetoManoDerecha) OtherActor)
    (Utilities|FlowControl|Sequence
      (:then_0
        (Variables|Default|SetPuedeAgarrarDerecha false))
      (:then_1
        (Variables|Default|SetobjetoManoDerecha 0)))))

(event OnComponentEndOverlap(BoxGrabLeft)
  (params (OverlappedComponent :type Primitive%20Component%20Object%20Reference) (OtherActor :type Actor%20Object%20Reference) (OtherComp :type Primitive%20Component%20Object%20Reference) (OtherBodyIndex :type Integer))
  (if (== (Variables|Default|GetobjetoManoIzquierda) OtherActor)
    (Utilities|FlowControl|Sequence
      (:then_0
        (Variables|Default|SetPuedeAgarrarIzquierda false))
      (:then_1
        (Variables|Default|SetobjetoManoIzquierda 0)))))

(event Input|EnhancedActionEvents|EnhancedInputActionia_move
  (params (ActionValue :type Vector :default "0, 0, 0") (ElapsedSeconds :type Float%20%28double-precision%29) (TriggeredSeconds :type Float%20%28double-precision%29) (InputAction :type Input%20Action%20Object%20Reference :default "/Game/Game/core/input/ia_move.ia_move"))
  (bind _camera (Variables|Default|GetCamera))
  (Transformation|SetActorLocation (+ (Transformation|GetActorLocation) (.ReturnValue (Utilities|CalculoMovimiento (* (Math|Vector|GetForwardVector _camera) (.x ActionValue)))) (.ReturnValue (Utilities|CalculoMovimiento (* (Math|Vector|GetRightVector _camera) (.y ActionValue)))) (.ReturnValue (Utilities|CalculoMovimiento (* (Math|Vector|GetUpVector _camera) (.z ActionValue))))) false false))

(event Input|EnhancedActionEvents|EnhancedInputActionia_rotation
  (params (ActionValue :type Vector%202D%20Structure) (ElapsedSeconds :type Float%20%28double-precision%29) (TriggeredSeconds :type Float%20%28double-precision%29) (InputAction :type Input%20Action%20Object%20Reference :default "/Game/Game/core/input/ia_rotation.ia_rotation"))
  (bind _returnvalue (Utilities|Time|GetWorldDeltaSeconds))
  (bind _velocidadrotacion (Variables|Default|GetvelocidadRotacion))
  (bind _returnvalue_2 (* ActionValue _velocidadrotacion _returnvalue))
  (Transformation|AddRelativeRotation (Variables|Default|GetDefaultSceneRoot) (Math|Rotator|MakeRotator 0.0 (.y _returnvalue_2) (.x _returnvalue_2)) false false))

(event Input|EnhancedActionEvents|EnhancedInputActionia_moveRVX
  (params (ActionValue :type Float%20%28double-precision%29) (ElapsedSeconds :type Float%20%28double-precision%29) (TriggeredSeconds :type Float%20%28double-precision%29) (InputAction :type Input%20Action%20Object%20Reference :default "/Game/Game/core/input/ia_moveRVX.ia_moveRVX"))
  (Transformation|SetActorLocation (+ (Transformation|GetActorLocation) (.ReturnValue (Utilities|CalculoMovimiento (* ActionValue (Math|Vector|GetRightVector (Variables|Default|GetCamera)))))) false false))

(event Input|EnhancedActionEvents|EnhancedInputActionia_agarreDeManoIzquierda
  (params (ActionValue :type Boolean) (ElapsedSeconds :type Float%20%28double-precision%29) (TriggeredSeconds :type Float%20%28double-precision%29) (InputAction :type Input%20Action%20Object%20Reference :default "/Game/Game/core/input/ia_agarreDeManoIzquierda.ia_agarreDeManoIzquierda"))
  (if (not (Variables|Default|GetTieneObjetoIzquierda))
    (if (Variables|Default|GetPuedeAgarrarIzquierda)
      (if (Utilities|IsValid (Variables|Default|GetobjetoManoIzquierda))
        (Transformation|AttachComponentToComponent (Variables|Default|GetobjetoManoIzquierda) (Variables|Default|GetSphere) "None" "SnapToTarget" "SnapToTarget" "KeepWorld" true)
        (Utilities|FlowControl|Sequence
          (:then_0
            (Variables|Default|SetTieneObjetoIzquierda true))
          (:then_1
            (Variables|Default|SetobjetoManoIzquierdaAgarrado (Variables|Default|GetobjetoManoIzquierda))))))))

(event Input|EnhancedActionEvents|EnhancedInputActionia_agarreDeManoDerecha
  (params (ActionValue :type Boolean) (ElapsedSeconds :type Float%20%28double-precision%29) (TriggeredSeconds :type Float%20%28double-precision%29) (InputAction :type Input%20Action%20Object%20Reference :default "/Game/Game/core/input/ia_agarreDeManoDerecha.ia_agarreDeManoDerecha"))
  (if (not (Variables|Default|GetTieneObjetoDerecha))
    (if (Variables|Default|GetPuedeAgarrarDerecha)
      (if (Utilities|IsValid (Variables|Default|GetobjetoManoDerecha))
        (Utilities|FlowControl|Sequence
          (:then_0
            (Transformation|AttachComponentToComponent (Variables|Default|GetobjetoManoDerecha) (Variables|Default|GetSphere1) "None" "SnapToTarget" "SnapToTarget" "KeepWorld" true)
            (Utilities|FlowControl|Sequence
              (:then_0
                (Variables|Default|SetTieneObjetoDerecha true))
              (:then_1
                (Variables|Default|SetobjetoManoDerechaAgarrado (Variables|Default|GetobjetoManoDerecha)))))))
      (else
        (Development|PrintString "No PUEDE AGARRAR")))))

(event Input|EnhancedActionEvents|EnhancedInputActionia_moveRVY
  (params (ActionValue :type Float%20%28double-precision%29) (ElapsedSeconds :type Float%20%28double-precision%29) (TriggeredSeconds :type Float%20%28double-precision%29) (InputAction :type Input%20Action%20Object%20Reference :default "/Game/Game/core/input/ia_moveRVY.ia_moveRVY"))
  (Transformation|SetActorLocation (+ (.ReturnValue (Utilities|CalculoMovimiento (* (Math|Vector|GetForwardVector (Variables|Default|GetCamera)) ActionValue))) (Transformation|GetActorLocation)) false false))

(event Input|EnhancedActionEvents|EnhancedInputActionia_LanzarYdisparar
  (params (ActionValue :type Boolean) (ElapsedSeconds :type Float%20%28double-precision%29) (TriggeredSeconds :type Float%20%28double-precision%29) (InputAction :type Input%20Action%20Object%20Reference :default "/Game/Game/core/input/ia_LanzarYdisparar.ia_LanzarYdisparar"))
  (if (Utilities|IsValid (Variables|Default|GetobjetoManoIzquierdaAgarrado))
    (if (Variables|Default|GetTieneObjetoIzquierda)
      (bind _asbp_hacha (Utilities|Casting|CastTobp_hacha (Variables|Default|GetobjetoManoIzquierdaAgarrado))
        (:then
          (Default|LanzarHacha _asbp_hacha)
          (Utilities|FlowControl|Sequence
            (:then_0
              (Variables|Default|SetTieneObjetoIzquierda false))
            (:then_1
              (Variables|Default|SetobjetoManoIzquierda 0))
            (:then_2
              (Variables|Default|SetobjetoManoIzquierdaAgarrado 0))))
        (:CastFailed
          (bind _asbp_revolver (Utilities|Casting|CastTobp_revolver (Variables|Default|GetobjetoManoIzquierdaAgarrado)))
          (Default|LanzarHacha _asbp_revolver)
          (Utilities|FlowControl|Sequence
            (:then_0
              (Variables|Default|SetTieneObjetoIzquierda false))
            (:then_1
              (Variables|Default|SetobjetoManoIzquierda 0))
            (:then_2
              (Variables|Default|SetobjetoManoIzquierdaAgarrado 0))))))))

(event Input|EnhancedActionEvents|EnhancedInputActionia_LanzarYdisparar
  (params (ActionValue :type Boolean) (ElapsedSeconds :type Float%20%28double-precision%29) (TriggeredSeconds :type Float%20%28double-precision%29) (InputAction :type Input%20Action%20Object%20Reference :default "/Game/Game/core/input/ia_LanzarYdisparar.ia_LanzarYdisparar"))
  (if (Utilities|IsValid (Variables|Default|GetobjetoManoDerechaAgarrado))
    (if (Variables|Default|GetTieneObjetoDerecha)
      (bind _asbp_hacha (Utilities|Casting|CastTobp_hacha (Variables|Default|GetobjetoManoDerechaAgarrado))
        (:then
          (Default|LanzarHacha _asbp_hacha)
          (Utilities|FlowControl|Sequence
            (:then_0
              (Variables|Default|SetTieneObjetoDerecha false))
            (:then_1
              (Variables|Default|SetobjetoManoDerecha 0))
            (:then_2
              (Variables|Default|SetobjetoManoDerechaAgarrado 0))))
        (:CastFailed
          (bind _asbp_revolver (Utilities|Casting|CastTobp_revolver (Variables|Default|GetobjetoManoDerechaAgarrado)))
          (Default|LanzarHacha _asbp_revolver)
          (Utilities|FlowControl|Sequence
            (:then_0
              (Variables|Default|SetTieneObjetoDerecha false))
            (:then_1
              (Variables|Default|SetobjetoManoDerecha 0))
            (:then_2
              (Variables|Default|SetobjetoManoDerechaAgarrado 0))))))))

(fn ConstructionScript)