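; Duck target that glides along the Y axis and awards points when struck, with a 15-second lifespan.
; Tick adds VelocidadMovimiento to its Y position each frame, without delta-time scaling.
; When an actor tagged "Golpeador" overlaps Ratacollision, it adds Valorrata to Bp_puntuacion, found via GetAllActorsOfClass.
; The hit also spawns an actor at a randomly lowered offset, plays a quack and shortens the lifespan to one second.
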(event OnComponentBeginOverlap(ratacollision)
  (params (OverlappedComponent :type Primitive%20Component%20Object%20Reference) (OtherActor :type Actor%20Object%20Reference) (OtherComp :type Primitive%20Component%20Object%20Reference) (OtherBodyIndex :type Integer) (bFromSweep :type Boolean) (SweepResult :type Hit%20Result%20Structure%20%28by%20ref%29))
  (bind _returnvalue (Transformation|GetActorLocation))
  ;[1 1 1] Si colisiona un objeto con tag de golpeador aumento la puntuacion emito un sonido y ademas creo un objeto hit y elimino el pato despues de 1 segundo
  (if (Actor|ActorHasTag OtherActor "Golpeador")
    (bind _outactors (Actor|GetAllActorsOfClass "/Game/Game/gameplay/bp_puntuacion.bp_puntuacion_C"))
    (Default|AumentarPuntuacion _outactors (Variables|Default|Getvalorrata))
    (Development|PrintString "Mas 5 punto")
    (Game|SpawnActorfromClass "/Game/Game/gameplay/bp_textoHIT.bp_textoHIT_C" (Math|Transform|MakeTransform (Math|Vector|MakeVector (+ (.x _returnvalue) 35.0) (.y _returnvalue) (- (.z _returnvalue) (Math|Random|RandomFloatinRange 1e+01 1.3e+02))) "0, 0, 0" "1.000000,1.000000,1.000000") "Undefined" "MultiplyWithRoot" 0 0)
    (Audio|PlaySoundatLocation "/Game/ModelosPropios/sonidos/404238__rafash1306__graznido-2.404238__rafash1306__graznido-2" (Transformation|GetActorLocation) "0, 0, 0" 0.5 1.0 0.0 0 0 0 0)
    (Actor|SetLifeSpan 1.0)))

(event EventBeginPlay
  ;[1 1 1] Le doy 15 segundos de vida al pato
  (Actor|SetLifeSpan 15.0))

(event Collision|EventActorBeginOverlap
  (params (OtherActor :type Actor%20Object%20Reference)))

(event EventTick
  (params (DeltaSeconds :type Float%20%28single-precision%29))
  (bind _returnvalue (Transformation|GetActorLocation))
  ;[1 1 1] Aumento la posicion en y del pato para que se mueva
  (Transformation|SetActorLocation (Math|Vector|MakeVector (.x _returnvalue) (.y (+ (Math|Vector|MakeVector 0.0 (.y _returnvalue) 0.0) (Variables|Default|GetvelocidadMovimiento))) (.z _returnvalue)) false false))

(fn ConstructionScript)