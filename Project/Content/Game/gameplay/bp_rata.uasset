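; Rat actor that wanders at random and awards score when hit by an actor tagged "Golpeador".
; ElegirNuevoDestino picks a random XY offset from the current location; Tick turns the rat's yaw toward it and moves with VInterpTo, repicking within a distance threshold.
; A tagged overlap on Ratacollision passes Valorrata to AumentarPuntuacion on Bp_puntuacion actors found via GetAllActorsOfClass and prints a message; the rat is not destroyed.
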(event OnComponentBeginOverlap(ratacollision)
  (params (OverlappedComponent :type Primitive%20Component%20Object%20Reference) (OtherActor :type Actor%20Object%20Reference) (OtherComp :type Primitive%20Component%20Object%20Reference) (OtherBodyIndex :type Integer) (bFromSweep :type Boolean) (SweepResult :type Hit%20Result%20Structure%20%28by%20ref%29))
  (if (Actor|ActorHasTag OtherActor "Golpeador")
    (bind _outactors (Actor|GetAllActorsOfClass "/Game/Game/gameplay/bp_puntuacion.bp_puntuacion_C"))
    (Default|AumentarPuntuacion _outactors (Variables|Default|Getvalorrata))
    (Development|PrintString "Mas 5 punto")))

(event EventBeginPlay
  (CallFunction|ElegirNuevoDestino))

(event Collision|EventActorBeginOverlap
  (params (OtherActor :type Actor%20Object%20Reference)))

(event EventTick
  (params (DeltaSeconds :type Float%20%28single-precision%29))
  (bind _returnvalue (Transformation|GetActorLocation))
  (bind _destinoactual (Variables|Default|GetdestinoActual))
  (if (Variables|Default|Getbmoviendo)
    (Transformation|SetActorRotation (Math|Rotator|MakeRotator 0.0 0.0 (.Yaw (Math|Rotator|BreakRotator (Math|Rotator|FindLookatRotation _returnvalue _destinoactual)))))
    (Transformation|SetActorLocation (Math|Interpolation|VInterpTo _returnvalue _destinoactual DeltaSeconds (Variables|Default|GetvelocidadMovimiento)) false false)
    (if (<= (Math|Vector|Distance(Vector) _returnvalue _destinoactual) (Variables|Default|GetumbralDistancia))
      (Variables|Default|Setbmoviendo false)
      (CallFunction|ElegirNuevoDestino))))

(fn ConstructionScript)

(fn ElegirNuevoDestino
  (bind _rangomovimiento (Variables|Default|GetrangoMovimiento))
  (bind _rangomovimiento2 (Variables|Default|GetrangoMovimiento2))
  (Variables|Default|SetdestinoActual (+ (Transformation|GetActorLocation) (Math|Vector|MakeVector (Math|Random|RandomFloatinRange _rangomovimiento2 _rangomovimiento) (Math|Random|RandomFloatinRange _rangomovimiento2 _rangomovimiento) 0.0)))
  (Variables|Default|Setbmoviendo true))