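; Ingot (lingote) Blueprint that acts as a hit target, awarding score when its Box is overlapped by an actor tagged "Golpeador".
; A valid overlap finds Bp_puntuacion through GetAllActorsOfClass and calls AumentarPuntuacion with ValorMuneco.
; It also prints a debug point message and spawns a Bp_textoHIT actor slightly offset from its own location as hit feedback.
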(event OnComponentBeginOverlap(Box)
  (params (OverlappedComponent :type Primitive%20Component%20Object%20Reference) (OtherActor :type Actor%20Object%20Reference) (OtherComp :type Primitive%20Component%20Object%20Reference) (OtherBodyIndex :type Integer) (bFromSweep :type Boolean) (SweepResult :type Hit%20Result%20Structure%20%28by%20ref%29))
  (bind _returnvalue (Transformation|GetActorLocation))
  (if (Actor|ActorHasTag OtherActor "Golpeador")
    (bind _outactors (Actor|GetAllActorsOfClass "/Game/Game/gameplay/bp_puntuacion.bp_puntuacion_C"))
    (Default|AumentarPuntuacion _outactors (Variables|Default|GetvalorMuneco))
    (Development|PrintString "Mas 1 punto")
    (Game|SpawnActorfromClass "/Game/Game/gameplay/bp_textoHIT.bp_textoHIT_C" (Math|Transform|MakeTransform (Math|Vector|MakeVector (+ (.x _returnvalue) 35.0) (.y _returnvalue) (- (.z _returnvalue) (Math|Random|RandomFloatinRange 1e+01 1e+01))) "0, 0, 0" "1.000000,1.000000,1.000000") "Undefined" "MultiplyWithRoot" 0 0)))

(event EventBeginPlay)

(event Collision|EventActorBeginOverlap
  (params (OtherActor :type Actor%20Object%20Reference)))

(event EventTick
  (params (DeltaSeconds :type Float%20%28single-precision%29)))

(fn ConstructionScript)