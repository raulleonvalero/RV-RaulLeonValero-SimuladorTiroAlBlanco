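; Rat spawner actor that creates a Bp_rata at its Arrow's location on BeginPlay and replaces it three seconds after it is destroyed.
; The first rat's OnDestroyed event triggers the initial respawn and sets SegundaVez.
; From then on, Tick polls the current rat's Muerta state and binds its destruction to a second handler, which repeats the delayed respawn.
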(event Custom|CustomEvent_1
  (params (DestroyedActor :type Actor%20Object%20Reference))
  ;[1 1 1] Esto hace lo mismo que la de arriba, pero añado una variable que comprueba que no es la primera vez, porque la funcion de arriba solo se hace cuando se crea el objeto, esta se hace a cada rato con el event tick
  (Variables|Default|SetrataActual 0)
  (Utilities|FlowControl|Delay 3.0)
  (bind _returnvalue (Game|SpawnActorfromClass "/Game/Game/gameplay/bp_rata.bp_rata_C" (Math|Conversions|ToTransform(Vector) (Transformation|GetWorldLocation (Variables|Default|GetArrow))) "Undefined" "MultiplyWithRoot" 0 0))
  (Variables|Default|SetrataActual _returnvalue))

(event Custom|rataMuerta
  (params (DestroyedActor :type Actor%20Object%20Reference))
  ;[1 1 1] Crea una rata nada mas empezar el juego, depues, espera hasta que la rata esta muerta y cuando es asi, esta desaparece despues de 3segundos y haber echo un sonido y crea otra rata nueva
  (Utilities|FlowControl|Delay 3.0)
  (bind _returnvalue (Game|SpawnActorfromClass "/Game/Game/gameplay/bp_rata.bp_rata_C" (Math|Conversions|ToTransform(Vector) (Transformation|GetWorldLocation (Variables|Default|GetArrow))) "Undefined" "MultiplyWithRoot" 0 0))
  (Variables|Default|SetrataActual _returnvalue)
  (Variables|Default|SetsegundaVez true))

(event EventBeginPlay
  ;[1 1 1] Crea una rata nada mas empezar el juego, depues, espera hasta que la rata esta muerta y cuando es asi, esta desaparece despues de 3segundos y haber echo un sonido y crea otra rata nueva
  (bind _returnvalue (Game|SpawnActorfromClass "/Game/Game/gameplay/bp_rata.bp_rata_C" (Math|Conversions|ToTransform(Vector) (Transformation|GetWorldLocation (Variables|Default|GetArrow))) "Undefined" "MultiplyWithRoot" 0 0))
  (bind _output_get (Variables|Default|SetrataActual _returnvalue))
  (Game|BindEventtoOnDestroyed _output_get (delegate Custom|rataMuerta)))

(event Collision|EventActorBeginOverlap
  (params (OtherActor :type Actor%20Object%20Reference))
  ;[1 1 1] Crea una rata nada mas empezar el juego, depues, espera hasta que la rata esta muerta y cuando es asi, esta desaparece despues de 3segundos y haber echo un sonido y crea otra rata nueva
)

(event EventTick
  (params (DeltaSeconds :type Float%20%28single-precision%29))
  (bind _rataactual (Variables|Default|GetrataActual))
  ;[1 1 1] Esto hace lo mismo que la de arriba, pero añado una variable que comprueba que no es la primera vez, porque la funcion de arriba solo se hace cuando se crea el objeto, esta se hace a cada rato con el event tick
  (if (Variables|Default|GetsegundaVez)
    (bind _asbp_rata (Utilities|Casting|CastTobp_rata _rataactual))
    (bind _newparam (Default|GetMuerta _asbp_rata))
    (if _newparam
      (Game|BindEventtoOnDestroyed _rataactual (delegate Custom|CustomEvent_1)))))

(fn ConstructionScript)