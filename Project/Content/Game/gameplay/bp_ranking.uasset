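; Ranking Blueprint that keeps and displays a top-five leaderboard of integer scores.
; AnadirPuntuacion adds a score while the list has room, or replaces the fifth entry when the new score is higher.
; After each insertion it sorts the array in descending order and calls ActualizarMarcador, which writes each entry to its text element, Primero through Quinto.
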(event EventBeginPlay)

(event Collision|EventActorBeginOverlap
  (params (OtherActor :type Actor%20Object%20Reference)))

(event EventTick
  (params (DeltaSeconds :type Float%20%28single-precision%29)))

(fn ConstructionScript)

(fn AnadirPuntuacion
  (params (puntuacion :type Integer))
  (bind _ranking (Variables|Default|GetRanking))
  (bind _ranking_2 (Variables|Default|GetRanking))
  (if (< (Utilities|Array|Length _ranking) 5)
    (Utilities|Array|Add _ranking_2 puntuacion :!label _label)
    (Class|KismetArrayLibrary|SortIntArray _ranking_2 false "Descending")
    (CallFunction|ActualizarMarcador)
    (else
      (for (_array_element _array_index) _ranking
        (if (== _array_index 4)
          (if (< _array_element puntuacion)
            (Utilities|Array|RemoveIndex _ranking 4)
            (goto _label)))))))

(fn ActualizarMarcador
  (for (_array_element _array_index) (Variables|Default|GetRanking)
    (if (== _array_index 0)
      (Rendering|Components|TextRender|SetText (Variables|Default|GetPrimero) (Utilities|Text|ToText(Integer) _array_element false true 1 1000))
      (elif (== _array_index 1)
        (Rendering|Components|TextRender|SetText (Variables|Default|Getsegundo) (Utilities|Text|ToText(Integer) _array_element false true 1 1000))
        (elif (== _array_index 2)
          (Rendering|Components|TextRender|SetText (Variables|Default|Gettercero) (Utilities|Text|ToText(Integer) _array_element false true 1 1000))
          (elif (== _array_index 3)
            (Rendering|Components|TextRender|SetText (Variables|Default|Getcuarto) (Utilities|Text|ToText(Integer) _array_element false true 1 1000))
            (elif (== _array_index 4)
              (Rendering|Components|TextRender|SetText (Variables|Default|Getquinto) (Utilities|Text|ToText(Integer) _array_element false true 1 1000)))))))))