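; Weapon spawner actor whose CreaArmas function, meant to run when the bell is touched, lays out weapons along X from its location.
; It spawns fixed sets of revolvers, axes and bottles, each in its own, mostly randomized X offset band.
; Three further slots each roll a weighted random pick among axe, revolver and bottle.
; The first random slot's final branch has no class set, where the others spawn a bottle.
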(event EventBeginPlay)

(event Collision|EventActorBeginOverlap
  (params (OtherActor :type Actor%20Object%20Reference)))

(event EventTick
  (params (DeltaSeconds :type Float%20%28single-precision%29)))

(fn ConstructionScript)

(fn CreaArmas
  (bind _returnvalue (Transformation|GetActorLocation))
  (bind _returnvalue_2 (Math|Random|RandomFloatinRange 4.9e+02 5e+02))
  (bind _returnvalue_3 (Transformation|GetActorLocation))
  (bind _returnvalue_4 (Transformation|GetActorLocation))
  (bind _returnvalue_5 (Math|Random|RandomFloatinRange 4.2e+02 4.5e+02))
  (bind _returnvalue_6 (Transformation|GetActorLocation))
  (bind _returnvalue_7 (Transformation|GetActorLocation))
  (bind _returnvalue_8 (Transformation|GetActorLocation))
  (bind _returnvalue_9 (Transformation|GetActorLocation))
  (bind _returnvalue_10 (Transformation|GetActorLocation))
  (bind _returnvalue_11 (Transformation|GetActorLocation))
  (bind _returnvalue_12 (Math|Random|RandomFloatinRange 3.5e+02 4e+02))
  (bind _returnvalue_13 (Transformation|GetActorLocation))
  (bind _returnvalue_14 (+ (.x _returnvalue) _returnvalue_2))
  (bind _returnvalue_15 (+ (.x _returnvalue_8) _returnvalue_12))
  (bind _returnvalue_16 (+ (.x _returnvalue_4) _returnvalue_5))
  ;[1 1 1] esta funcion crea las armas al tocar la campana
  (Utilities|FlowControl|Sequence
    (:then_0
      ;[1 1 1] Se CREAN LOS REVOLVEREs, 2 en este caso
      (for _index (range 1 2)
        (if (== _index 1)
          (Game|SpawnActorfromClass "/Game/Game/gameplay/bp_revolver.bp_revolver_C" (Math|Transform|MakeTransform (Math|Vector|MakeVector (+ (.x _returnvalue_6) (Math|Random|RandomFloatinRange 0.0 0.0)) (.y _returnvalue_6) (.z _returnvalue_6)) "0, 0, 0" "1.000000,1.000000,1.000000") "Undefined" "MultiplyWithRoot" 0 0)
          (else
            (Game|SpawnActorfromClass "/Game/Game/gameplay/bp_revolver.bp_revolver_C" (Math|Transform|MakeTransform (Math|Vector|MakeVector (+ (.x _returnvalue_7) (Math|Random|RandomFloatinRange 5e+01 8e+01)) (.y _returnvalue_7) (.z _returnvalue_7)) "0, 0, 0" "1.000000,1.000000,1.000000") "Undefined" "MultiplyWithRoot" 0 0)))))
    (:then_1
      ;[1 1 1] Crea las hachas, 3 en este caso
      (for _index_2 (range 1 3)
        (if (== _index_2 1)
          (Game|SpawnActorfromClass "/Game/Game/gameplay/bp_hacha.bp_hacha_C" (Math|Transform|MakeTransform (Math|Vector|MakeVector (+ (.x _returnvalue_9) (Math|Random|RandomFloatinRange 1e+02 1.2e+02)) (.y _returnvalue_9) (.z _returnvalue_9)) "0, 0, 0" "1.000000,1.000000,1.000000") "Undefined" "MultiplyWithRoot" 0 0)
          (elif (== _index_2 2)
            (Game|SpawnActorfromClass "/Game/Game/gameplay/bp_hacha.bp_hacha_C" (Math|Transform|MakeTransform (Math|Vector|MakeVector (+ (.x _returnvalue_10) (Math|Random|RandomFloatinRange 1.5e+02 2e+02)) (.y _returnvalue_10) (.z _returnvalue_10)) "0, 0, 0" "1.000000,1.000000,1.000000") "Undefined" "MultiplyWithRoot" 0 0)
            (else
              (Game|SpawnActorfromClass "/Game/Game/gameplay/bp_hacha.bp_hacha_C" (Math|Transform|MakeTransform (Math|Vector|MakeVector (+ (.x _returnvalue_11) (Math|Random|RandomFloatinRange 2.2e+02 2.5e+02)) (.y _returnvalue_11) (.z _returnvalue_11)) "0, 0, 0" "1.000000,1.000000,1.000000") "Undefined" "MultiplyWithRoot" 0 0))))))
    (:then_2
      ;[1 1 1] Crea las botellas, 2 en este caso
      (for _index_3 (range 1 2)
        (if (== _index_3 1)
          (Game|SpawnActorfromClass "/Game/Game/gameplay/bp_botella.bp_botella_C" (Math|Transform|MakeTransform (Math|Vector|MakeVector (+ (.x _returnvalue_13) (Math|Random|RandomFloatinRange 2.7e+02 3e+02)) (.y _returnvalue_13) (.z _returnvalue_13)) "0, 0, 0" "1.000000,1.000000,1.000000") "Undefined" "MultiplyWithRoot" 0 0)
          (else
            (Game|SpawnActorfromClass "/Game/Game/gameplay/bp_botella.bp_botella_C" (Math|Transform|MakeTransform (Math|Vector|MakeVector (+ (.x _returnvalue_3) (Math|Random|RandomFloatinRange 3.2e+02 3.3e+02)) (.y _returnvalue_3) (.z _returnvalue_3)) "0, 0, 0" "1.000000,1.000000,1.000000") "Undefined" "MultiplyWithRoot" 0 0)))))
    (:then_3
      ;[1 1 1 1 69] Esta parte se encarga de generar tres objetos, pueden ser tres objetos diferentes una hacha, un revolver o una botella, esta logica se encarga de generar uno u otro de forma aleatoria
      (for _index_4 (range 1 3)
        (if (== _index_4 1)
          (bind _output_get (Variables|Default|Setprobabilidad (Math|Random|RandomFloatinRange 0.0 1.0)))
          (if (<= _output_get 0.4)
            (Game|SpawnActorfromClass "/Game/Game/gameplay/bp_hacha.bp_hacha_C" (Math|Transform|MakeTransform (Math|Vector|MakeVector _returnvalue_15 (.y _returnvalue_8) (.z _returnvalue_8)) "0, 0, 0" "1.000000,1.000000,1.000000") "Undefined" "MultiplyWithRoot" 0 0)
            (elif (<= _output_get 0.7)
              (Game|SpawnActorfromClass "/Game/Game/gameplay/bp_revolver.bp_revolver_C" (Math|Transform|MakeTransform (Math|Vector|MakeVector _returnvalue_15 (.y _returnvalue_8) (.z _returnvalue_8)) "0, 0, 0" "1.000000,1.000000,1.000000") "Undefined" "MultiplyWithRoot" 0 0)
              (else
                (Game|SpawnActorfromClass "/Game/Game/gameplay/bp_botella.bp_botella_C" (Math|Transform|MakeTransform (Math|Vector|MakeVector _returnvalue_15 (.y _returnvalue_8) (.z _returnvalue_8)) "0, 0, 0" "1.000000,1.000000,1.000000") "Undefined" "MultiplyWithRoot" 0 0))))
          (elif (== _index_4 2)
            (bind _output_get_2 (Variables|Default|Setprobabilidad (Math|Random|RandomFloatinRange 0.0 1.0)))
            (if (<= _output_get_2 0.4)
              (Game|SpawnActorfromClass "/Game/Game/gameplay/bp_hacha.bp_hacha_C" (Math|Transform|MakeTransform (Math|Vector|MakeVector _returnvalue_16 (.y _returnvalue_4) (.z _returnvalue_4)) "0, 0, 0" "1.000000,1.000000,1.000000") "Undefined" "MultiplyWithRoot" 0 0)
              (elif (<= _output_get_2 0.7)
                (Game|SpawnActorfromClass "/Game/Game/gameplay/bp_revolver.bp_revolver_C" (Math|Transform|MakeTransform (Math|Vector|MakeVector _returnvalue_16 (.y _returnvalue_4) (.z _returnvalue_4)) "0, 0, 0" "1.000000,1.000000,1.000000") "Undefined" "MultiplyWithRoot" 0 0)
                (else
                  (Game|SpawnActorfromClass "/Game/Game/gameplay/bp_botella.bp_botella_C" (Math|Transform|MakeTransform (Math|Vector|MakeVector _returnvalue_16 (.y _returnvalue_4) (.z _returnvalue_4)) "0, 0, 0" "1.000000,1.000000,1.000000") "Undefined" "MultiplyWithRoot" 0 0))))
            (else
              (bind _output_get_3 (Variables|Default|Setprobabilidad (Math|Random|RandomFloatinRange 0.0 1.0)))
              (if (<= _output_get_3 0.4)
                (Game|SpawnActorfromClass "/Game/Game/gameplay/bp_hacha.bp_hacha_C" (Math|Transform|MakeTransform (Math|Vector|MakeVector _returnvalue_14 (.y _returnvalue) (.z _returnvalue)) "0, 0, 0" "1.000000,1.000000,1.000000") "Undefined" "MultiplyWithRoot" 0 0)
                (elif (<= _output_get_3 0.7)
                  (Game|SpawnActorfromClass "/Game/Game/gameplay/bp_revolver.bp_revolver_C" (Math|Transform|MakeTransform (Math|Vector|MakeVector _returnvalue_14 (.y _returnvalue) (.z _returnvalue)) "0, 0, 0" "1.000000,1.000000,1.000000") "Undefined" "MultiplyWithRoot" 0 0)
                  (else
                    (Game|SpawnActorfromClass "/Game/Game/gameplay/bp_botella.bp_botella_C" (Math|Transform|MakeTransform (Math|Vector|MakeVector _returnvalue_14 (.y _returnvalue) (.z _returnvalue)) "0, 0, 0" "1.000000,1.000000,1.000000") "Undefined" "MultiplyWithRoot" 0 0)))))))))))