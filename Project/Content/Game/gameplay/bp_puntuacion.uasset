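; Score keeper Blueprint that holds the running point total and displays it in game through its Puntuacion text.
; Functions add to, reset and return PuntosTotales, while Tick rewrites the text from that total every frame.
; AcabaPuntuacion hands the final total to the Bp_ranking actors, found with GetAllActorsOfClass, by calling AnadirPuntuacion on them.
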(event EventBeginPlay)

(event Collision|EventActorBeginOverlap
  (params (OtherActor :type Actor%20Object%20Reference)))

(event EventTick
  (params (DeltaSeconds :type Float%20%28single-precision%29))
  (Rendering|Components|TextRender|SetText (Variables|Default|Getpuntuacion) (Utilities|Text|ToText(Integer) (Variables|Default|GetpuntosTotales))))

(fn ConstructionScript)

(fn AumentarPuntuacion
  (params (NewParam :type Integer))
  (Variables|Default|SetpuntosTotales (+ NewParam (Variables|Default|GetpuntosTotales))))

(fn ResetearPuntuacion
  (Variables|Default|SetpuntosTotales 0))

(fn GetPuntuacion
  (return (Variables|Default|GetpuntosTotales)))

(fn AcabaPuntuacion
  (bind _outactors (Actor|GetAllActorsOfClass "/Game/Game/gameplay/bp_ranking.bp_ranking_C"))
  (Default|AnadirPuntuacion _outactors (Variables|Default|GetpuntosTotales)))