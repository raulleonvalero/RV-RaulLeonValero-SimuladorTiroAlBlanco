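; Bell actor (campana) that lets the player end and reset the scoring when a hand rings it.
; Overlap events on the Campana component set an EstaTocando flag while an actor tagged "mano" is touching it.
; TocaCampana, which nothing in this Blueprint calls, checks that flag, then finds the Bp_puntuacion actors and calls AcabaPuntuacion followed by ResetearPuntuacion.
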(event OnComponentBeginOverlap(campana)
  (params (OverlappedComponent :type Primitive%20Component%20Object%20Reference) (OtherActor :type Actor%20Object%20Reference) (OtherComp :type Primitive%20Component%20Object%20Reference) (OtherBodyIndex :type Integer) (bFromSweep :type Boolean) (SweepResult :type Hit%20Result%20Structure%20%28by%20ref%29))
  (if (Actor|ActorHasTag OtherActor "mano")
    (Variables|Default|SetestaTocando true)))

(event OnComponentEndOverlap(campana)
  (params (OverlappedComponent :type Primitive%20Component%20Object%20Reference) (OtherActor :type Actor%20Object%20Reference) (OtherComp :type Primitive%20Component%20Object%20Reference) (OtherBodyIndex :type Integer))
  (if (Actor|ActorHasTag OtherActor "mano")
    (Variables|Default|SetestaTocando false)))

(event EventBeginPlay)

(event Collision|EventActorBeginOverlap
  (params (OtherActor :type Actor%20Object%20Reference)))

(event EventTick
  (params (DeltaSeconds :type Float%20%28single-precision%29)))

(fn ConstructionScript)

(fn TocaCampana
  (if (Variables|Default|GetestaTocando)
    (Utilities|FlowControl|Sequence
      (:then_0
        (bind _outactors (Actor|GetAllActorsOfClass "/Game/Game/gameplay/bp_puntuacion.bp_puntuacion_C"))
        (Default|AcabaPuntuacion _outactors)
        (Default|ResetearPuntuacion _outactors)))))